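; BP_StartSwitch is a gaze-activated cube that starts the game when looked at long enough, then destroys itself.
; GazeTrigger highlights the cube through custom depth and counts down GazeTime, choosing which side to show.
; RotateCube lerps between sides on a timeline, ignoring calls mid-turn; reaching side zero sets IsGameStarted on PlayerMode.
; A looping CheckForReset timer clears the highlight and resets the countdown and side when gaze lapses.
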(event `RotateCube`
  (params (CurrentSec :type Integer))
  (bind _rotatesides (`self.RotateSides`))
  ;[1 1 1] Rotate Cube
  (if (not (`self.IsLerping`))
    (set `self.PreviousSide` (`self.CurrentSide`))
    (set `self.CurrentSide` CurrentSec)
    (set `self.IsLerping` true)
    (bind (_direction _cubelerp) (`Timeline|Gazetracer_TimeLine` :!via `PlayFromStart`)
      (:`Update`
        (`self.K2_SetActorRotation` (`KismetMathLibrary.RLerp` (`KismetArrayLibrary.Array_Get` _rotatesides (`self.PreviousSide`)) (`KismetArrayLibrary.Array_Get` _rotatesides (`self.CurrentSide`)) _cubelerp)))
      (:`Finished`
        (set `self.IsLerping` false)
        (if (== (`self.CurrentSide`) 0)
          (bind _asplayer_mode (cast `/Game/Blueprints/PlayerMode` (`GameplayStatics.GetGameMode`)))
          (set `/Game/Blueprints/PlayerMode.IsGameStarted` true _asplayer_mode)
          (`KismetSystemLibrary.K2_SetTimerDelegate` (delegate `DestroySelf`) 2.0))))))

(event `DestroySelf`
  (`self.K2_DestroyActor`))

(event `self.ReceiveBeginPlay`
  (set `self.GazeTime` (`self.MaxGazeTime`))
  (set `self.TimeToReset` (`self.MaxTimeToReset`))
  (`KismetSystemLibrary.K2_SetTimer` null "CheckForReset" 0.05 true))

(event `self.GazeTrigger`
  (`PrimitiveComponent.SetRenderCustomDepth` (`self.Cube`) true)
  (set `self.TimeToReset` (`self.MaxTimeToReset`))
  (bind _output_get (set `self.GazeTime` (- (`self.GazeTime`) (`GameplayStatics.GetWorldDeltaSeconds`))))
  (if (< _output_get 0.0)
    (`self.RotateCube` 0)
    (elif (< _output_get 1.0)
      (`self.RotateCube` 1)
      (elif (< _output_get 2.0)
        (`self.RotateCube` 2)))))

(event `self.ReceiveTick`
  (params (DeltaSeconds :type "Float (single-precision)")))

(event `OnGazeReset`
  ;[1 1 1] ResetCube
  (set `self.GazeTime` (`self.MaxGazeTime`))
  (`self.RotateCube` 3))

(fn `CheckForReset`
  (bind _output_get (set `self.TimeToReset` (- (`self.TimeToReset`) (`KismetSystemLibrary.K2_GetTimerElapsedTime` null "CheckForReset"))))
  (if (< _output_get 0.0)
    (`self.OnGazeReset`)
    (elif (< _output_get (- (`self.MaxTimeToReset`) 0.1))
      (`PrimitiveComponent.SetRenderCustomDepth` (`self.Cube`) false))))

(fn `UserConstructionScript`
  (`parent.UserConstructionScript`))