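; BP_Spacebox is an actor, likely a space backdrop going by its name, that follows the player pawn along the world X axis.
; A looping 0.1-second timer started on BeginPlay moves it to the pawn's X position while keeping its own Y and Z, instead of updating on Tick.
; Each update prints the SetActorLocation success result to screen as debug output.
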(event `self.ReceiveBeginPlay`
  (`KismetSystemLibrary.K2_SetTimerDelegate` (delegate `FollowPlayer`) 0.1 true))

(event `FollowPlayer`
  (bind (_sweephitresult _returnvalue) (`self.K2_SetActorLocation` (`KismetMathLibrary.MakeVector` (.x (`self.K2_GetActorLocation` (`GameplayStatics.GetPlayerPawn` 0))) (.y (`self.K2_GetActorLocation`)) (.z (`self.K2_GetActorLocation`)))))
  (`KismetSystemLibrary.PrintString` (`KismetStringLibrary.Conv_BoolToString` _returnvalue)))

(event `self.ReceiveTick`
  (params (DeltaSeconds :type "Float (single-precision)")))

(fn `UserConstructionScript`)