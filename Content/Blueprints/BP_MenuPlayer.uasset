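; BP_MenuPlayer is the menu player, with gaze-based interaction driven by its Camera.
; Every Tick calls GazeCounter, which line traces a long distance along the camera's forward vector.
; When the trace hits a BP_GazeModificableObject, it calls GazeTrigger on that object each frame, leaving the response to the object itself.
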(event `self.ReceiveTick`
  (params (DeltaSeconds :type "Float (single-precision)"))
  (`self.GazeCounter` 200000.0))

(fn `GazeCounter`
  (params (TraceLength :type "Float (double-precision)"))
  (bind _camera (`self.Camera`))
  (bind _returnvalue (`SceneComponent.K2_GetComponentLocation` _camera))
  (bind (_outhit _returnvalue_2) (`KismetSystemLibrary.LineTraceSingle` _returnvalue (+ _returnvalue (* (`SceneComponent.GetForwardVector` _camera) TraceLength)) "TraceTypeQuery3"))
  (if _returnvalue_2
    (bind _asbp_gaze_modificable_object (cast `/Game/GazeModificableObject/BP_GazeModificableObject` (`.HitActor` (`GameplayStatics.BreakHitResult` _outhit))))
    (`/Game/GazeModificableObject/BP_GazeModificableObject.GazeTrigger` _asbp_gaze_modificable_object)))

(fn `UserConstructionScript`)