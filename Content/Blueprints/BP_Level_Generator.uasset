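; Level generator that builds an endless run of lane actors, spawning a start switch and initial lanes on BeginPlay.
; Each lane is picked randomly from Beginner or Easy arrays by a randomized progress-versus-threshold check, then chained along negative X by lane length.
; Past ten on the counter, which spawns also increment, checkpoint passes trim old lanes, spawn new ones and raise global time dilation, an experimental speedup flagged risky for VR.
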(event `OnCheckpointPass`
  ;[1 1 1] Invoked on passing a checkpoint, deletes passed lanes and spawnes further ones, also increases time flow
  (bind _result (`/Engine/EditorBlueprintResources/StandardMacros.IncrementInt` (`self.CurrentCheckpointId`))
    (:`  `
      (if (> _result 10)
        (`self.DeleteOldestLane`)
        (`self.SpawnNextLane`)
        ;;[1 1 1] !!Experimental!! !!Dangerous on VR!! additive speedup
        (`GameplayStatics.SetGlobalTimeDilation` (+ (`GameplayStatics.GetGlobalTimeDilation`) (`self.SpeedupPerCheckpoint`)))))))

(event `self.ReceiveBeginPlay`
  (`self.GenerateLevel`))

(fn `DeleteOldestLane`
  (bind _spawnedobjects (`self.SpawnedObjects`))
  (bind _item (`KismetArrayLibrary.Array_Get` _spawnedobjects))
  (`KismetArrayLibrary.Array_RemoveItem` _spawnedobjects _item)
  (`self.K2_DestroyActor` _item)
  (return))

(fn `DestroyWholeLevel`
  (bind _spawnedobjects (`self.SpawnedObjects`))
  (for _array_element _spawnedobjects
    (`self.K2_DestroyActor` _array_element))
  (`KismetArrayLibrary.Array_Clear` _spawnedobjects))

(fn `GenerateLevel`
  ;[1 1 1] Generate the beginning part of level
  ;;[1 1 1] ResetLevelProgress
  (set `self.CurrentCheckpointId` 0)
  (set `self.NextSpawnPos` (struct))
  (`GameplayStatics.SetGlobalTimeDilation` 1.0)
  (`|SpawnActorFromClass` "/Game/GazeModificableObject/BP_StartSwitch.BP_StartSwitch_C" (`self.StartSwitchTransform`) "Undefined" "OverrideRootScale")
  (for _ (range (+ (`self.MaxSpawnAmount`) 1))
    (`self.SpawnNextLane`)))

(fn `SpawnNextLane`
  (bind _returnvalue (* (`self.CurrentCheckpointId`) (`KismetMathLibrary.RandomIntegerInRange` 3 12)))
  (if (and (>= _returnvalue (`self.BeginnerLaneSpawnThreshold`)) (< _returnvalue (`self.EasyLaneSpawnThreshold`)))
    (`self.SpawnNextLaneFromLanesArray` (`self.BeginnerLanes`))
    (elif true
      (`self.SpawnNextLaneFromLanesArray` (`self.EasyLanes`)))))

(fn `SpawnNextLaneFromLanesArray`
  (params (LevelLanes :type "Array of /Game/LevelLanes/BP_Level_Lane Class Reference (by ref)"))
  (bind _returnvalue (`|SpawnActorFromClass` (`self.RandomElement` LevelLanes) (`self.NextSpawnPos`) "AdjustIfPossibleButAlwaysSpawn" "OverrideRootScale"))
  (`KismetArrayLibrary.Array_Add` (`self.SpawnedObjects`) _returnvalue)
  (`/Engine/EditorBlueprintResources/StandardMacros.IncrementInt` (`self.CurrentCheckpointId`)
    (:`  `
      (set `self.NextSpawnPos` (`self.GetNextLanePosition` _returnvalue)))))

(fn `UserConstructionScript`)