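; PlayerMode sets up the generated level at startup and streams its lanes as checkpoint progress advances.
; On BeginPlay it spawns a LevelGenerator at the world origin, stores the reference and calls GenerateLevel.
; CheckpointIdUpdate increments the current checkpoint ID and, once past a small threshold, has the generator delete the oldest lane and spawn the next, forming a rolling window of track.
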(event `self.ReceiveBeginPlay`
  ;[1 1 1] Generate Level
  (bind _returnvalue (`|SpawnActorFromClass` (`self.LevelGenerator`) (`KismetMathLibrary.MakeTransform` (0.0 0.0 0.0)) "Undefined" "OverrideRootScale"))
  (set `self.LevelGeneratorReference` _returnvalue)
  (`/Game/LevelLanes/BP_Level_Generator.GenerateLevel` _returnvalue)
  (`KismetSystemLibrary.PrintString` "SUCCESS"))

(fn `CheckpointIdUpdate`
  (bind _levelgeneratorreference (`self.LevelGeneratorReference`))
  (bind _result (`/Engine/EditorBlueprintResources/StandardMacros.IncrementInt` (`self.CurrentCheckpointId`))
    (:`  `
      (if (> _result 5)
        (`/Game/LevelLanes/BP_Level_Generator.DeleteOldestLane` _levelgeneratorreference)
        (`/Game/LevelLanes/BP_Level_Generator.SpawnNextLane` _levelgeneratorreference)))))

(fn `UserConstructionScript`)