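; BP_Score is an actor that tracks the player's score and pushes it to the Score widget on the player pawn.
; On BeginPlay it registers with PlayerMode, starts a looping timer and caches the widget.
; While the game is started, each timer tick adds the multiplier scaled by global time dilation, compounding the multiplier whenever dilation exceeds its last recorded value.
; A ResetScore event restores score, multiplier and recorded dilation.
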(event `self.ReceiveBeginPlay`
  (bind _asplayer_mode (cast `/Game/Blueprints/PlayerMode` (`GameplayStatics.GetGameMode`)))
  (bind _output_get (set `self.GameModeReference` _asplayer_mode))
  (set `/Game/Blueprints/PlayerMode.BP_ScoreReference` self _output_get)
  ;[1 1 1] Set timer for updating the score
  (`KismetSystemLibrary.K2_SetTimerDelegate` (delegate `SetScore`) (`self.ScoreTimer`) true)
  ;[1 1 1] Set Player and ScoreWidget variables
  (bind _asplayer (cast `/Game/Blueprints/Player` (`GameplayStatics.GetPlayerPawn` 0))
    (:`then`
      (bind _output_get_2 (set `self.PlayerReference` _asplayer))
      (bind _asscore (cast `/Game/UI/Score` (`WidgetComponent.GetUserWidgetObject` (`/Game/Blueprints/Player.ScoreWidget` _output_get_2)))
        (:`then`
          (set `self.ScoreWidget` _asscore))
        (:`CastFailed`
          (`KismetSystemLibrary.PrintString` "retard"))))
    (:`CastFailed`
      (`KismetSystemLibrary.PrintString` "Wrong player class!"))))

(event `SetScore`
  (bind _returnvalue (`GameplayStatics.GetGlobalTimeDilation`))
  (bind _returnvalue_2 (`KismetMathLibrary.FTrunc` (* (`self.ScoreMultiplier`) _returnvalue)))
  ;[1 1 1] Set score and update multiplier
  (if (`/Game/Blueprints/PlayerMode.IsGameStarted` (`self.GameModeReference`))
    (bind _output_get (set `self.Score` (+ (`self.Score`) _returnvalue_2)))
    (if (> _returnvalue (`self.LastDilation`))
      (set `self.ScoreMultiplier` _returnvalue_2)
      (set `self.LastDilation` _returnvalue))
    (`/Game/UI/Score.ChangeScore` (`self.ScoreWidget`) _output_get)))

(event `ResetScore`
  (set `self.LastDilation` 0.0)
  (set `self.ScoreMultiplier` 10)
  (bind _output_get (set `self.Score` 0))
  (`/Game/UI/Score.ChangeScore` (`self.ScoreWidget`) _output_get))

(fn `UserConstructionScript`)